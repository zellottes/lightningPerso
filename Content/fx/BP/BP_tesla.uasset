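; Tesla effect actor that fires Niagara lightning beams at the player while they are inside its SphereCol trigger.
; Overlap starts a looping timer that adds a new beam component from the Sphere's relative location to the player's spine_01 socket; leaving clears it.
; BeginPlay also loops a timer on spawnNiagaraSytem, but that function's random-endpoint beam logic is disconnected, so it does nothing.
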(event `self.ReceiveBeginPlay`
  (`KismetSystemLibrary.K2_SetTimer` null "spawnNiagaraSytem" 0.1 true))

(event `self.SphereCol.OnComponentBeginOverlap`
  (params (OverlappedComponent :type "PrimitiveComponent Object Reference") (OtherActor :type "Actor Object Reference") (OtherComp :type "PrimitiveComponent Object Reference") (OtherBodyIndex :type Integer) (bFromSweep :type Boolean) (SweepResult :type "HitResult Structure (by ref)"))
  (if (== OtherActor (`GameplayStatics.GetPlayerCharacter` 0))
    (bind _returnvalue (`KismetSystemLibrary.K2_SetTimerDelegate` (delegate `CustomEvent`) 0.5 true))
    (set `self.mytimer` _returnvalue)))

(event `CustomEvent`
  (`self.StartPlayerLighting`))

(event `StartPlayerLighting`
  (bind _returnvalue (`AddComponent|NODE_AddNiagaraComponent-2`))
  (`NiagaraComponent.SetVariableVec3` _returnvalue "BeamStart" (`SceneComponent.RelativeLocation` (`self.Sphere`)))
  (`NiagaraComponent.SetVariableVec3` _returnvalue "BeamEnd" (`SceneComponent.GetSocketLocation` (`Character.Mesh` (`GameplayStatics.GetPlayerCharacter` 0)) "spine_01")))

(event `self.SphereCol.OnComponentEndOverlap`
  (params (OverlappedComponent :type "PrimitiveComponent Object Reference") (OtherActor :type "Actor Object Reference") (OtherComp :type "PrimitiveComponent Object Reference") (OtherBodyIndex :type Integer))
  (if (== OtherActor (`GameplayStatics.GetPlayerCharacter` 0))
    (`KismetSystemLibrary.K2_ClearAndInvalidateTimerHandle` (`self.mytimer`))))

(fn `spawnNiagaraSytem`)

(fn `UserConstructionScript`)